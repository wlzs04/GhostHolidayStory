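; StoryCoverContainer_BP turns horizontal input into browsing between story covers.
; On BeginPlay it casts the first player pawn to MainPawn_BP and caches it.
; The Right input axis calls ShowNextStoryCover on that pawn at full positive deflection and ShowLastStoryCover at full negative.
; It has no debounce of its own, so a held input repeats the call on each axis event.
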(event `self.ReceiveBeginPlay`
  (bind _asmain_pawn_bp (cast `/Game/GameContent/Manager/MainPawn_BP` (`GameplayStatics.GetPlayerPawn` 0)))
  (set `self.mainPawn` _asmain_pawn_bp))

(event `InputAxis|Right`
  (params (AxisValue :type "Float (single-precision)"))
  (bind _mainpawn (`self.mainPawn`))
  (if (>= AxisValue 1.0)
    (`/Game/GameContent/Manager/MainPawn_BP.ShowNextStoryCover` _mainpawn)
    (elif (<= AxisValue -1.0)
      (`/Game/GameContent/Manager/MainPawn_BP.ShowLastStoryCover` _mainpawn))))

(fn `UserConstructionScript`)