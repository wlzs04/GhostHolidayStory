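; Story cover actor that displays a 2D sprite as a story's cover, sized to a portrait 1:1.414 (A-series paper) ratio.
; The construction script derives the width from the cover height and scales a backing sprite to fit, which is hidden on BeginPlay.
; SetStorySprite swaps in the cover image and scales it from its component bounds using the same width and height.
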(event `self.ReceiveBeginPlay`
  (`SceneComponent.SetVisibility` (`self.BackSprite`) false false))

(fn `SetStorySprite`
  (params (storySprite :type "PaperSprite Object Reference"))
  (bind _storycoversprite (`self.StoryCoverSprite`))
  (`PaperSpriteComponent.SetSprite` _storycoversprite storySprite)
  (`SceneComponent.SetRelativeScale3D` _storycoversprite (`KismetMathLibrary.MakeVector` (/ (`self.coverWidth`) (.y (`.BoxExtent` (`KismetSystemLibrary.GetComponentBounds` _storycoversprite)))) 1.0 (/ (`self.civerHeight`) (.z (`.BoxExtent` (`KismetSystemLibrary.GetComponentBounds` _storycoversprite)))))))

(fn `UserConstructionScript`
  (bind _backsprite (`self.BackSprite`))
  ;[1 1 1] 设置封面的宽高
  (set `self.coverWidth` (/ (`self.civerHeight`) 1.414))
  ;[1 1 1] 设置背景的大小
  (`SceneComponent.SetRelativeScale3D` _backsprite (`KismetMathLibrary.MakeVector` (/ (`self.coverWidth`) (.y (`.BoxExtent` (`KismetSystemLibrary.GetComponentBounds` _backsprite)))) 1.0 (/ (`self.civerHeight`) (.z (`.BoxExtent` (`KismetSystemLibrary.GetComponentBounds` _backsprite)))))))