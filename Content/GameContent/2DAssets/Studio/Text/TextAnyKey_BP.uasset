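; Actor that animates "Any Key" prompt letters along a circle until OpenDoor dismisses it.
; NormalTimeLine drives the angle of five text render components spaced 45 degrees apart, while GetTransfromByRadius converts each angle to a relative Y/Z position using Radius.
; OpenDoor stops that timeline and plays OpenDoorTimeLine, which adds its track to the last angle for a continuous exit motion, then destroys the actor.
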(event `self.ReceiveBeginPlay`
  (bind _tempvalue (`self.tempValue`))
  (`|ExecutionSequence`
    (:`then_0`
      (bind (_direction `_新建轨迹_0`) (`Timeline|openDoorTimeLine` :!via `Stop`)
        (:`Update`
          (`|ExecutionSequence`
            (:`then_0`
              (bind _returnvalue (+ `_新建轨迹_0` (`self.tempValue`)))
              (`self.GetTransfromByRadius` (+ _returnvalue 0.0) (`self.TextRender_A`)))
            (:`then_1`
              (`self.GetTransfromByRadius` (+ _returnvalue 45.0) (`self.TextRender_n`)))
            (:`then_2`
              (`self.GetTransfromByRadius` (+ _returnvalue 90.0) (`self.TextRender_y`)))
            (:`then_3`
              (`self.GetTransfromByRadius` (+ _returnvalue 135.0) (`self.TextRender_e`)))
            (:`then_4`
              (`self.GetTransfromByRadius` (+ _returnvalue 180.0) (`self.TextRender_K`)))))
        (:`Finished`
          (`self.K2_DestroyActor`))))
    (:`then_1`
      (bind (_direction_2 `_新建轨迹_0_2`) (`Timeline|normalTimeLine`)
        (:`Update`
          (set `self.tempValue` `_新建轨迹_0_2`)
          (`|ExecutionSequence`
            (:`then_0`
              (`self.GetTransfromByRadius` _tempvalue (`self.TextRender_A`)))
            (:`then_1`
              (`self.GetTransfromByRadius` (+ _tempvalue 45.0) (`self.TextRender_n`)))
            (:`then_2`
              (`self.GetTransfromByRadius` (+ _tempvalue 90.0) (`self.TextRender_y`)))
            (:`then_3`
              (`self.GetTransfromByRadius` (+ _tempvalue 135.0) (`self.TextRender_e`)))
            (:`then_4`
              (`self.GetTransfromByRadius` (+ _tempvalue 180.0) (`self.TextRender_K`)))))))))

(fn `GetTransfromByRadius`
  (params (value :type "Float (double-precision)") (textRender :type "TextRenderComponent Object Reference"))
  (bind _radius (`self.radius`))
  (`SceneComponent.K2_SetRelativeLocation` textRender (`KismetMathLibrary.MakeVector` 0.0 (* (- 0.0 (`KismetMathLibrary.DegSin` value)) _radius) (* (`KismetMathLibrary.DegCos` value) _radius)) false false)
  (return))

(fn `OpenDoor`
  (`TimelineComponent.Stop` (`self.normalTimeLine`))
  (`TimelineComponent.Play` (`self.openDoorTimeLine`)))

(fn `UserConstructionScript`)