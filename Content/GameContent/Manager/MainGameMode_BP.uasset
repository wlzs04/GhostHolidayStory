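; Main game mode Blueprint that applies the configured audio volumes to the game's sound classes.
; InitSoundBPEvent overrides the background, voice and special sound classes in MainSoundMix with no fade, each set to the CommonConfig total volume multiplied by that category's volume.
; BeginPlay, Tick and the construction script contain no logic, and nothing in this graph calls the sound event.
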(event `self.ReceiveBeginPlay`)

(event `self.InitSound_BPEvent`
  (bind _commonconfig (`self.commonConfig`))
  (bind _commonconfig_2 (`self.commonConfig`))
  (bind _commonconfig_3 (`self.commonConfig`))
  (`|ExecutionSequence`
    (:`then_0`
      (`GameplayStatics.SetSoundMixClassOverride` "/Game/GameContent/Manager/UserData/Sound/MainSoundMix.MainSoundMix" "/Game/GameContent/Manager/UserData/Sound/Back_SoundClass.Back_SoundClass" (* (`CommonConfig.totalVolume` _commonconfig_2) (`CommonConfig.backVolume` _commonconfig_2)) 1.0 0.0))
    (:`then_1`
      (`GameplayStatics.SetSoundMixClassOverride` "/Game/GameContent/Manager/UserData/Sound/MainSoundMix.MainSoundMix" "/Game/GameContent/Manager/UserData/Sound/Voice_SoundClass.Voice_SoundClass" (* (`CommonConfig.totalVolume` _commonconfig_3) (`CommonConfig.voiceVolume` _commonconfig_3)) 1.0 0.0))
    (:`then_2`
      (`GameplayStatics.SetSoundMixClassOverride` "/Game/GameContent/Manager/UserData/Sound/MainSoundMix.MainSoundMix" "/Game/GameContent/Manager/UserData/Sound/Special_SoundClass.Special_SoundClass" (* (`CommonConfig.totalVolume` _commonconfig) (`CommonConfig.specialVolume` _commonconfig)) 1.0 0.0))))

(fn `UserConstructionScript`)