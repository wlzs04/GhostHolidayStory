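; MainPawn_BP is the main pawn that plays the sequence of entering the studio through a door.
; On BeginPlay it finds the door sprite, its attached AnyKey text actor and the flashlight spotlight by actor label.
; EnterStudioBPEvent starts the text actor's OpenDoor and a door-rotation timeline.
; That timeline's event destroys the flashlight, moves the pawn along X through a second timeline and prints a random greeting from MainGameMode.
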(event `self.ReceiveBeginPlay`
  (`self.IntActor`))

(event `self.EnterStudio_BPEvent`
  ;[1 1 1] 播放门把手旋转动画
  (`/Game/GameContent/2DAssets/Studio/Text/TextAnyKey_BP.OpenDoor` (`self.anyKeyTextActor`))
  ;[1 1 1] 播放开门动画
  (bind (_direction `_新建轨迹_0`) (`Timeline|openDoorTimeline`)
    (:`Update`
      (`self.SetDoorAngle` `_新建轨迹_0`))
    (:`事件`
      (`|ExecutionSequence`
        (:`then_0`
          ;[1 1 1] 关掉手电筒
          (`self.CloseFlashLight`))
        (:`then_1`
          ;[1 1 1] 进入门内
          (bind (_direction_2 `_新建轨迹_0_2`) (`Timeline|enterDoorTimeline`)
            (:`Update`
              (`self.K2_SetActorLocation` (`KismetMathLibrary.MakeVector` `_新建轨迹_0_2` 0.0 -30.0)))))
        (:`then_2`
          ;[1 1 1] 说一声问候语。
          (`self.SpeekGreetings`))))))

(fn `CloseFlashLight`
  (bind _spotlight (`self.spotLight`))
  ;[1 1 1] 关掉手电筒
  (if (`KismetSystemLibrary.IsValid` _spotlight)
    (`self.K2_DestroyActor` _spotlight)))

(fn `IntActor`
  (`|ExecutionSequence`
    (:`then_0`
      ;[1 1 1] 获得门Actor和门上的文字AnyKey
      (bind _outactors (`GameplayStatics.GetAllActorsOfClass` "/Script/Paper2D.PaperSpriteActor"))
      (for _array_element _outactors
        (if (`KismetStringLibrary.EqualEqual_StrStr` (`self.GetActorLabel` _array_element) "Door_Sprite")
          (bind _output_get (set `self.doorActor` _array_element))
          (for _array_element_2 (`self.GetAttachedActors` _output_get)
            (if (`KismetStringLibrary.EqualEqual_StrStr` (`self.GetActorLabel` _array_element_2) "TextAnyKey_BP")
              (bind _astext_any_key_bp (cast `/Game/GameContent/2DAssets/Studio/Text/TextAnyKey_BP` _array_element_2))
              (set `self.anyKeyTextActor` _astext_any_key_bp))))))
    (:`then_1`
      ;[1 1 1] 获得手电筒
      (bind _outactors_2 (`GameplayStatics.GetAllActorsOfClass` "/Script/Engine.SpotLight"))
      (for _array_element_3 _outactors_2
        (if (`KismetStringLibrary.EqualEqual_StrStr` (`self.GetActorLabel` _array_element_3) "FlashLight")
          (set `self.spotLight` _array_element_3))))))

(fn `SetDoorAngle`
  (params (currentTime :type "Float (double-precision)"))
  (`self.K2_SetActorRelativeRotation` (`self.doorActor`) (`KismetMathLibrary.MakeRotator` 0.0 0.0 currentTime) false false))

(fn `SpeekGreetings`
  (bind _returnvalue (`GhostHolidayStoryGameModeBase.GetRandomGreetingsTalkGroup` (`self.mainGameMode`)))
  (`KismetSystemLibrary.PrintString` (`.text` (break `TextAndAudio` (`.talk0` (break `TalkGroup` _returnvalue))))))

(fn `UserConstructionScript`)